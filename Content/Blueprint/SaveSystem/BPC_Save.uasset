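; Save component that keeps a leaderboard of up to five dated score and time records in a save slot.
; SaveData appends while there is room; once full, it replaces the last entry only if the new score-per-time ratio is at least as high.
; Each change is re-sorted via SortGameData before saving.
; LoadData returns the records as parallel date, score and formatted-time arrays for display.
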(event EventBeginPlay)

(event EventTick
  (params (DeltaSeconds :type Float%20%28single-precision%29)))

(fn SaveData
  (params (Score :type Float%20%28single-precision%29) (Time :type Float%20%28single-precision%29))
  ;[1 1 1] Is Save Size is more than 5?
  (LocalVariables|SetScoreToSave Score)
  (LocalVariables|SetTimeToSave Time)
  (bind _gamedata (CallFunction|LoadGame (Variables|Default|GetSave%20Slot)))
  (bind _output_get (LocalVariables|SetGameData _gamedata))
  (if (>= (Utilities|Array|Length _output_get) 5)
    ;[1 1 1] True: Calculate Avg Score To Save
    (bind _avgscore (CallFunction|CalculateAvgScore (LocalVariables|GetScoreToSave) (LocalVariables|GetTimeToSave)))
    (LocalVariables|SetAvgToSave _avgscore)
    (bind _avgscore_2 (CallFunction|CalculateAvgScore (.Score (Utilities|Struct|BreakS_GameData (Utilities|Array|Get(acopy) (LocalVariables|GetGameData) (Utilities|Array|LastIndex (LocalVariables|GetGameData))))) (.Time (Utilities|Struct|BreakS_GameData (Utilities|Array|Get(acopy) (LocalVariables|GetGameData) (Utilities|Array|LastIndex (LocalVariables|GetGameData)))))))
    (LocalVariables|SetAvgLoaded _avgscore_2)
    (if (>= (LocalVariables|GetAvgToSave) (LocalVariables|GetAvgLoaded))
      ;[1 1 1] If new score is higher, save the score and remove previous score
      (bind _gamedata_2 (CallFunction|CreateGameData (LocalVariables|GetScoreToSave) (LocalVariables|GetTimeToSave)))
      (bind _returnvalue (Utilities|Array|Add (LocalVariables|GetGameData) _gamedata_2))
      (Utilities|Array|RemoveIndex (LocalVariables|GetGameData) (- _returnvalue 1))
      (bind _sortedgamedata (CallFunction|SortGameData (LocalVariables|GetGameData)))
      (CallFunction|SaveGame _sortedgamedata (Variables|Default|GetSave%20Slot))
      (return)
      (else
        (return)))
    (else
      ;[1 1 1] False: Immediately save game data
      (bind _gamedata_3 (CallFunction|CreateGameData (LocalVariables|GetScoreToSave) (LocalVariables|GetTimeToSave)))
      (Utilities|Array|Add (LocalVariables|GetGameData) _gamedata_3)
      (bind _sortedgamedata_2 (CallFunction|SortGameData (LocalVariables|GetGameData)))
      (CallFunction|SaveGame _sortedgamedata_2 (Variables|Default|GetSave%20Slot))
      (return))))

(fn CreateGameData
  (params (Score :type Float%20%28single-precision%29) (Time :type Float%20%28single-precision%29))
  (return (Utilities|Struct|MakeS_GameData (Math|DateTime|Now) Score Time)))

(fn CalculateAvgScore
  (params (Score :type Float%20%28single-precision%29) (Time :type Float%20%28single-precision%29))
  (return (/ Score Time)))

(fn LoadData
  (Utilities|Array|Clear (LocalVariables|GetDateArray))
  (Utilities|Array|Clear (LocalVariables|GetScoreArray))
  (Utilities|Array|Clear (LocalVariables|GetTimeArray))
  (bind _gamedata (CallFunction|LoadGame (Variables|Default|GetSave%20Slot)))
  (for _array_element _gamedata
    (bind _formattedtext (CallFunction|FormatTime (.Time (Utilities|Struct|BreakS_GameData _array_element))))
    (Utilities|Array|Add (LocalVariables|GetTimeArray) _formattedtext)
    (Utilities|Array|Add (LocalVariables|GetDateArray) (Class|KismetTextLibrary|AsDateDateTime (.Date (Utilities|Struct|BreakS_GameData _array_element))))
    (Utilities|Array|Add (LocalVariables|GetScoreArray) (Utilities|Text|ToText(Float) (.Score (Utilities|Struct|BreakS_GameData _array_element)) "HalfToEven")))
  (return (LocalVariables|GetDateArray) (LocalVariables|GetScoreArray) (LocalVariables|GetTimeArray)))