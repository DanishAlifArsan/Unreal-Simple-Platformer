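; Blueprint function library for saving and loading a GameData payload through BP_SaveGame objects in enum-named slots, all under user index 0.
; SaveGame checks whether the slot exists, loading it or creating a new save object, then passes the data to SaveToSlot to write.
; LoadGame returns the stored GameData through LoadFromSlot, whose IsLoad flag controls whether data is returned alongside the save reference.
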(fn InitializeSaveSystem
  (bind _returnvalue (SaveGame|CreateSaveGameObject "/Game/Blueprint/SaveSystem/BP_SaveGame.BP_SaveGame_C"))
  (return _returnvalue))

(fn SavetoSlot
  (params (GameData :type Array%20of%20S%20Game%20Data%20Structures) (SaveRef :type BP%20Save%20Game%20Object%20Reference) (SaveSlot :type String))
  (Variables|/Game/Blueprint/SaveSystem/BP_SaveGame.BP_SaveGame_C|SetGameData SaveRef GameData)
  (SaveGame|SaveGametoSlot SaveRef SaveSlot))

(fn LoadfromSlot
  (params (IsLoad :type Boolean) (SaveSlot :type String))
  (LocalVariables|SetIsActualLoad IsLoad)
  (bind _returnvalue (SaveGame|LoadGamefromSlot SaveSlot))
  (bind _asbp_save_game (Utilities|Casting|CastToBP_SaveGame _returnvalue))
  (if (LocalVariables|GetIsActualLoad)
    (return (Variables|/Game/Blueprint/SaveSystem/BP_SaveGame.BP_SaveGame_C|GetGameData _asbp_save_game) _asbp_save_game)
    (else
      (return 0 _asbp_save_game))))

(fn SaveGame
  (params (GameData :type Array%20of%20S%20Game%20Data%20Structures) (SaveSlot :type E_SaveSlot%20Enum :default "NewEnumerator0"))
  (bind _returnvalue (Utilities|String|EnumtoString SaveSlot))
  (LocalVariables|SetDataToSave GameData)
  (LocalVariables|SetSlotToSave _returnvalue)
  (bind _returnvalue_2 (SaveGame|DoesSaveGameExist _returnvalue))
  (if _returnvalue_2
    (bind _saveref (CallFunction|LoadfromSlot false (LocalVariables|GetSlotToSave)))
    (else
      (bind _saveref_2 (CallFunction|InitializeSaveSystem))))
  (CallFunction|SavetoSlot (LocalVariables|GetDataToSave) _saveref_2 (LocalVariables|GetSlotToSave) _saveref))

(fn LoadGame
  (params (SaveSlot :type E_SaveSlot%20Enum :default "NewEnumerator0"))
  (bind _gamedata (CallFunction|LoadfromSlot true (Utilities|String|EnumtoString SaveSlot)))
  (return _gamedata))