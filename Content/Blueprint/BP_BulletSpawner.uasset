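; BP_BulletSpawner is an actor that fires Bullet actors repeatedly on a timer.
; BeginPlay starts a looping timer that runs SpawnBullet every Interval.
; Each shot spawns a bullet at the spawner's transform, calls its SetLifetime, then calls MoveBullet with the X component of the root component's forward vector.
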(event Custom|SpawnBullet
  ;[1 1 1] SpawnBullet
  (bind _returnvalue (Game|SpawnActorfromClass (Variables|Default|GetBullet) (Transformation|GetActorTransform) "Undefined" 0 0))
  (Default|SetLifetime _returnvalue)
  (Default|MoveBullet _returnvalue (.X (Math|Vector|BreakVector (Math|Vector|GetForwardVector (Transformation|GetWorldRotation (Variables|Default|GetDefaultSceneRoot)))))))

(event EventBeginPlay
  ;[1 1 1] SpawnBullet
  (Utilities|Time|SetTimerbyEvent (delegate Custom|SpawnBullet) (Variables|Default|GetInterval) true))

(fn ConstructionScript)