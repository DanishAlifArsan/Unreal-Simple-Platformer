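; BFL_Utils is a Blueprint function library with helpers for formatting time and ranking game records.
; FormatTime converts seconds into "minute:second" text using floored division and modulo.
; SortGameData bubble-sorts GameData entries in descending order of score divided by time, stopping early when a pass makes no swaps, and returns the array.
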(fn FormatTime
  (params (Timer :type Float%20%28single-precision%29))
  (return (Utilities|Text|FormatText "{minute}:{second}" (Utilities|Text|ToText(Integer) (Math|Conversions|ToInteger(Byte) (Class|KismetMathLibrary|FFloor64 (/ Timer 6e+01))) false true 2 2) (Utilities|Text|ToText(Integer) (Math|Conversions|ToInteger(Byte) (Class|KismetMathLibrary|FFloor64 (Math|Float|%(Float) Timer 6e+01))) false true 2 2))))

(fn SortGameData
  (params (GameData :type Array%20of%20S%20Game%20Data%20Structures))
  (LocalVariables|SetDataToSort GameData)
  (bind _output_get (LocalVariables|SetCurrentIndex 0))
  (bind _index (Utilities|FlowControl|ForLoopwithBreak _output_get (Utilities|Array|LastIndex (LocalVariables|GetDataToSort)) :!label _label)
    (:LoopBody
      (LocalVariables|SetCurrentIndex _index)
      (LocalVariables|SetSwapped false)
      (bind _output_get_2 (LocalVariables|SetNextIndex 0))
      (bind _index_2 (Utilities|FlowControl|ForLoopwithBreak _output_get_2 (- (- (Utilities|Array|LastIndex (LocalVariables|GetDataToSort)) (LocalVariables|GetCurrentIndex)) 1))
        (:LoopBody
          (LocalVariables|SetNextIndex _index_2)
          (if (< (/ (.Score (Utilities|Struct|BreakS_GameData (Utilities|Array|Get(acopy) (LocalVariables|GetDataToSort) (LocalVariables|GetNextIndex)))) (.Time (Utilities|Struct|BreakS_GameData (Utilities|Array|Get(acopy) (LocalVariables|GetDataToSort) (LocalVariables|GetNextIndex))))) (/ (.Score (Utilities|Struct|BreakS_GameData (Utilities|Array|Get(acopy) (LocalVariables|GetDataToSort) (+ (LocalVariables|GetNextIndex) 1)))) (.Time (Utilities|Struct|BreakS_GameData (Utilities|Array|Get(acopy) (LocalVariables|GetDataToSort) (+ (LocalVariables|GetNextIndex) 1))))))
            (LocalVariables|SetTempData (Utilities|Array|Get(acopy) (LocalVariables|GetDataToSort) (LocalVariables|GetNextIndex)))
            (Utilities|Array|SetArrayElem (LocalVariables|GetDataToSort) (LocalVariables|GetNextIndex) (Utilities|Array|Get(acopy) (LocalVariables|GetDataToSort) (+ (LocalVariables|GetNextIndex) 1)))
            (Utilities|Array|SetArrayElem (LocalVariables|GetDataToSort) (+ (LocalVariables|GetNextIndex) 1) (LocalVariables|GetTempData))
            (LocalVariables|SetSwapped true)))
        (:Completed
          (if (not (LocalVariables|GetSwapped))
            (goto _label Break)))))
    (:Completed
      (return (LocalVariables|GetDataToSort)))))