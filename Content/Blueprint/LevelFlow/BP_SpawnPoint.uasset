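; BP_SpawnPoint is a checkpoint that the player activates by overlapping its collision.
; When a ThirdPersonCharacter enters while inactive, it marks itself active, registers itself with ThirdPersonGameMode via SetSpawnPoint, updates its text label and plays a 2D sound.
; A Deactivate event clears the active flag and resets the label, allowing the point to be activated again.
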(event OnComponentBeginOverlap(Collision)
  (params (OverlappedComponent :type Primitive%20Component%20Object%20Reference) (OtherActor :type Actor%20Object%20Reference) (OtherComp :type Primitive%20Component%20Object%20Reference) (OtherBodyIndex :type Integer) (bFromSweep :type Boolean) (SweepResult :type Hit%20Result%20Structure%20%28by%20ref%29))
  ;[1 1 1] Activate Spawn Point
  (Utilities|Casting|CastToThirdPersonCharacter OtherActor)
  (if (not (Variables|Default|GetIsActive))
    (Variables|Default|SetIsActive true)
    (bind _asthird_person_game_mode (Utilities|Casting|CastToThirdPersonGameMode (Game|GetGameMode)))
    (Default|SetSpawnPoint _asthird_person_game_mode self)
    (Rendering|Components|TextRender|SetText (Variables|Default|GetTextRender) (Utilities|Text|MakeLiteralText "Activated"))
    (Audio|PlaySound2D "/Game/Assets/Audio/SFX/Teleport_Cue.Teleport_Cue" 1.0 1.0 0.0 0 0)))

(event Custom|Deactivate
  ;[1 1 1] Deactivate Spawn Point
  (Variables|Default|SetIsActive false)
  (Rendering|Components|TextRender|SetText (Variables|Default|GetTextRender) (Utilities|Text|MakeLiteralText "Not Active")))

(fn ConstructionScript)