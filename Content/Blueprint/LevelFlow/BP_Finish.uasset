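; BP_Finish is a level finish trigger that ends the game when the ThirdPersonCharacter overlaps its collision.
; On overlap it calls GameEnded on ThirdPersonGameMode, copies the current time into game instance data and unpossesses the player controller.
; It then opens the W_GameOver widget and saves the coin amount and time from the game instance through BPCSave.
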(event OnComponentBeginOverlap(Collision)
  (params (OverlappedComponent :type Primitive%20Component%20Object%20Reference) (OtherActor :type Actor%20Object%20Reference) (OtherComp :type Primitive%20Component%20Object%20Reference) (OtherBodyIndex :type Integer) (bFromSweep :type Boolean) (SweepResult :type Hit%20Result%20Structure%20%28by%20ref%29))
  (bind _returnvalue (Game|GetPlayerController 0))
  ;[1 1 1] Gameover when player collider
  (Utilities|Casting|CastToThirdPersonCharacter OtherActor)
  (bind _asthird_person_game_mode (Utilities|Casting|CastToThirdPersonGameMode (Game|GetGameMode)))
  (Default|GameEnded _asthird_person_game_mode)
  (CallFunction|SetGameInstanceTimeData (Variables|/Game/ThirdPersonBP/Blueprints/ThirdPersonGameMode.ThirdPersonGameMode_C|GetCurrentTime _asthird_person_game_mode))
  (Pawn|UnPossess _returnvalue)
  (bind _returnvalue_2 (UserInterface|CreateWidget "/Game/Blueprint/HUD/W_GameOver.W_GameOver_C" _returnvalue))
  (UserInterface|Viewport|AddtoViewport _returnvalue_2 0)
  (Default|OpenMenu _returnvalue_2)
  (bind (_currenthealth _coinamount _maxhealth _time) (CallFunction|GetGameInstanceData))
  (Default|SaveData (Variables|Default|GetBPC_Save) _coinamount _time))

(fn ConstructionScript)